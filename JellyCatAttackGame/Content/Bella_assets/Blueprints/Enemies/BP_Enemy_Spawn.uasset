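; BP_Enemy_Spawn is an enemy spawner actor that links itself to the BP_Mission it sits in; it contains no spawning logic.
; Its construction script runs a small capsule overlap at its location, stores the first mission found and registers itself via AddEnemySpawnerMessage.
; When none is found, it unregisters from the stored mission and clears the reference, so the link updates as the actor is placed or reconstructed.
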(event EventBeginPlay)

(event Collision|EventActorBeginOverlap
  (params (OtherActor :type Actor%20Object%20Reference)))

(event EventTick
  (params (DeltaSeconds :type Float%20%28single-precision%29)))

(fn ConstructionScript
  (bind _self self)
  (bind _outactors (Collision|CapsuleOverlapActors (Transformation|GetActorLocation) 2e+01 0.0 (Variables|Default|GetObject%20Types) "/Game/Bella_assets/Blueprints/Missions/BP_Mission.BP_Mission_C"))
  (Utilities|IsValid (Utilities|Array|Get(acopy) _outactors)
    (:Is%20Valid
      (Variables|Default|SetMIssion%20Overlapped (Utilities|Array|Get(acopy) _outactors))
      (Class|BPIEnemySpawn|AddEnemySpawner(Message) (Utilities|Array|Get(acopy) _outactors) _self))
    (:Is%20Not%20Valid
      (Class|BPIEnemySpawn|RemoveEnemySpawner(Message) (Variables|Default|GetMIssion%20Overlapped) _self)
      (Variables|Default|SetMIssion%20Overlapped 0))))