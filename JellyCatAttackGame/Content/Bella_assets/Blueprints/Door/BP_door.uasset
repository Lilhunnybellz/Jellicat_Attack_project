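; BP_door is a door that swings open when a character enters its trigger box.
; The box overlap accepts actors implementing BPI_Character_Vals, unless the door is Locked or already opening.
; A Timeline lerps the Door component's relative yaw through a quarter turn, clearing IsOpening when finished.
; It has no closing logic, so a later overlap replays the swing from the closed angle.
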(event OnComponentBeginOverlap(Box)
  (params (OverlappedComponent :type Primitive%20Component%20Object%20Reference) (OtherActor :type Actor%20Object%20Reference) (OtherComp :type Primitive%20Component%20Object%20Reference) (OtherBodyIndex :type Integer) (bFromSweep :type Boolean) (SweepResult :type Hit%20Result%20Structure%20%28by%20ref%29))
  (if (Math|Boolean|ANDBoolean (Utilities|DoesObjectImplementInterface OtherActor "/Game/Variant_Shooter/Blueprints/Pickups/BPI_Character_Vals.BPI_Character_Vals_C") (not (Variables|Default|GetisOpening)) (not (Variables|Default|Getlocked)))
    (Variables|Default|SetisOpening true)
    (bind _door (Timeline|Timeline PlayFromStart)
      (:Update
        (Transformation|SetRelativeRotation (Variables|Default|Getdoor) (Math|Rotator|MakeRotator 0.0 0.0 (Math|Float|Lerp 0.0 -9e+01 _door)) false false))
      (:Finished
        (Variables|Default|SetisOpening false)))))

(event EventBeginPlay)

(event Collision|EventActorBeginOverlap
  (params (OtherActor :type Actor%20Object%20Reference)))

(event EventTick
  (params (DeltaSeconds :type Float%20%28single-precision%29)))

(fn ConstructionScript)