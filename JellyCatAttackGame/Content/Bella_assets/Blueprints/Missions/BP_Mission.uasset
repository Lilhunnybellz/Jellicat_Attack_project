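; BP_Mission is a mission actor that tracks a set of enemy spawners and a mission status.
; Its add and remove events update the SpawnPoints list and set or clear each spawner's ParentMission back-reference.
; When an actor implementing BPI_Character_Vals overlaps the Collision component, the status advances one state, provided it is in the required prior state.
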(event OnComponentBeginOverlap(Collision)
  (params (OverlappedComponent :type Primitive%20Component%20Object%20Reference) (OtherActor :type Actor%20Object%20Reference) (OtherComp :type Primitive%20Component%20Object%20Reference) (OtherBodyIndex :type Integer) (bFromSweep :type Boolean) (SweepResult :type Hit%20Result%20Structure%20%28by%20ref%29))
  (if (and (Utilities|DoesObjectImplementInterface OtherActor "/Game/Variant_Shooter/Blueprints/Pickups/BPI_Character_Vals.BPI_Character_Vals_C") (Utilities|Enum|Equal(Enum) (Variables|Default|GetMission%20Status) "NewEnumerator1"))
    (Variables|Default|SetMission%20Status "NewEnumerator2")))

(event EventBeginPlay)

(event Collision|EventActorBeginOverlap
  (params (OtherActor :type Actor%20Object%20Reference)))

(event EventTick
  (params (DeltaSeconds :type Float%20%28single-precision%29)))

(event EventRemoveEnemySpawner
  (params (Enemy%20Spawner :type BP%20Enemy%20Spawn%20Object%20Reference))
  (Utilities|Set|Remove (Variables|Default|GetSpawn%20Points) Enemy%20Spawner)
  (Variables|/Game/Bella_assets/Blueprints/Enemies/BP_Enemy_Spawn.BP_Enemy_Spawn_C|SetParent%20Mission Enemy%20Spawner 0))

(event EventAddEnemySpawner
  (params (Enemy%20Spawner :type BP%20Enemy%20Spawn%20Object%20Reference))
  (Utilities|Set|Add (Variables|Default|GetSpawn%20Points) Enemy%20Spawner)
  (Variables|/Game/Bella_assets/Blueprints/Enemies/BP_Enemy_Spawn.BP_Enemy_Spawn_C|SetParent%20Mission Enemy%20Spawner self))

(fn ConstructionScript)